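; BP_Place spawns small ice cubes at an iceberg and moves them toward a base.
; A looping timer spawns each scaled-down cube at a random offset along the iceberg's forward axis, ignoring Pawn collision, and stores it in AllCubes.
; Tick steps every valid cube horizontally toward Base and rotates it to face there.
; The step is per frame without delta time and divides by MoveSpeed, so higher values move cubes slower.
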(event `self.ReceiveTick`
  (params (DeltaSeconds :type "Float (single-precision)"))
  (for _array_element (`self.AllCubes`)
    (`/Engine/EditorBlueprintResources/StandardMacros.IsValid` _array_element
      (:`Is Valid`
        (bind _rootcomponent (`Actor.RootComponent` _array_element))
        (bind _returnvalue (`SceneComponent.K2_GetComponentLocation` _rootcomponent))
        (bind _returnvalue_2 (- (`SceneComponent.K2_GetComponentLocation` (`self.Base`)) _returnvalue))
        (`SceneComponent.K2_SetWorldLocation` _rootcomponent (`KismetMathLibrary.MakeVector` (.x (+ _returnvalue (/ _returnvalue_2 (* (`KismetMathLibrary.VSize` _returnvalue_2) (`KismetMathLibrary.Conv_IntToDouble` (`self.MoveSpeed`)))))) (.y (+ _returnvalue (/ _returnvalue_2 (* (`KismetMathLibrary.VSize` _returnvalue_2) (`KismetMathLibrary.Conv_IntToDouble` (`self.MoveSpeed`)))))) (.z _returnvalue)) false false)
        (`self.K2_SetActorRotation` _array_element (`KismetMathLibrary.FindLookAtRotation` _returnvalue (`SceneComponent.K2_GetComponentLocation` (`self.Base`))) false)))))

(event `self.ReceiveBeginPlay`
  (`KismetSystemLibrary.K2_SetTimerDelegate` (delegate `Spawn Cubes`) 3.0 true))

(event `Spawn Cubes`
  (bind _iceberg (`self.Iceberg`))
  (bind _returnvalue (`|SpawnActorFromClass` "/Game/Blueprints/IceCube.IceCube_C" (`KismetMathLibrary.MakeTransform` (+ (`SceneComponent.K2_GetComponentLocation` _iceberg) (* (`SceneComponent.GetForwardVector` _iceberg) (`KismetMathLibrary.RandomFloatInRange` -20.0 20.0)))) "AlwaysSpawn" "OverrideRootScale" null null))
  (`self.SetActorScale3D` _returnvalue (0.02 0.02 0.02))
  (`PrimitiveComponent.SetCollisionResponseToChannel` (`/Game/Blueprints/IceCube.IceCube` _returnvalue) "ECC_Pawn" "ECR_Ignore")
  (`KismetArrayLibrary.Array_Add` (`self.AllCubes`) _returnvalue))

(fn `UserConstructionScript`)